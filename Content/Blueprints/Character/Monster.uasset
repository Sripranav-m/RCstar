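; Zombie enemy that wanders, chases and attacks the player, and takes damage from projectiles.
; AIMoveTo loops drive random roaming and a sight-triggered chase, though sighting sets SeenPlayer false, leaving the roam loop unblocked.
; Reaching the player opens a timed attack window in which sphere overlap damages once.
; Projectile hits reduce health, update objective text, then either spawn impact fire and trigger pursuit, or ragdoll the zombie and count the kill.
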(event `self.ReceiveBeginPlay`
  (`|AIMoveTo` self (`NavigationSystemV1.K2_GetRandomReachablePointInRadius` (`self.K2_GetActorLocation`) 500.0 null null) null :!label _label
    (:`OnSuccess`
      _)
    (:`OnFail`
      _))
  (if (not (`self.seenPlayer`))
    (goto _label)))

(event `self.ReceiveActorBeginOverlap`
  (params (OtherActor :type "Actor Object Reference"))
  (bind _asprojectile_base (cast `/Game/Blueprints/Character_Weapons/projectile_base` OtherActor))
  (bind _asmain_character (cast `/Game/Blueprints/Character/mainCharacter` (`GameplayStatics.GetPlayerCharacter` 0)))
  (set `/Game/Blueprints/Character/mainCharacter.objectiveText` "Zombie has been damaged by 10%." _asmain_character)
  (set `self.health` (- (`self.health`) 0.1))
  (if (<= (`self.health`) 0.0)
    (bind _asmonster (cast `/Game/Blueprints/Character/Monster` self))
    (`PrimitiveComponent.SetSimulatePhysics` (`Character.Mesh` _asmonster) true)
    (bind _asmain_character_2 (cast `/Game/Blueprints/Character/mainCharacter` (`GameplayStatics.GetPlayerCharacter` 0)))
    (set `/Game/Blueprints/Character/mainCharacter.killedZombies` (+ (`/Game/Blueprints/Character/mainCharacter.killedZombies` _asmain_character_2) 1) _asmain_character_2)
    (set `/Game/Blueprints/Character/mainCharacter.objectiveText` "Congrats!.You have killed zombie and scored 1 point.   " _asmain_character_2)
    (else
      (`GameplayStatics.SpawnEmitterAtLocation` "/Game/InfinityBladeEffects/Effects/FX_Mobile/Fire/combat/P_Ranged_Firey_Impact.P_Ranged_Firey_Impact" (`self.K2_GetActorLocation` _asprojectile_base))
      (bind _asmain_character_3 (cast `/Game/Blueprints/Character/mainCharacter` (`GameplayStatics.GetPlayerCharacter` 0)))
      (`|AIMoveTo` self (0.0 0.0 0.0) _asmain_character_3))))

(event `self.PawnSensing.OnSeePawn`
  (params (Pawn :type "Pawn Object Reference"))
  (bind _asmain_character (cast `/Game/Blueprints/Character/mainCharacter` (`GameplayStatics.GetPlayerCharacter` 0)))
  (set `self.seenPlayer` false)
  (`|AIMoveTo` self (0.0 0.0 0.0) _asmain_character :!label _label_2
    (:`OnSuccess`
      (if (not (`self.attacking`))
        (set `self.attacking` true)
        (`KismetSystemLibrary.Delay` 2.3)
        (set `self.attacking` false)
        (set `self.alreadyHit` false)
        (goto _label_2)))))

(event `self.ReceiveTick`
  (params (DeltaSeconds :type "Float (single-precision)")))

(event `self.Sphere.OnComponentBeginOverlap`
  (params (OverlappedComponent :type "PrimitiveComponent Object Reference") (OtherActor :type "Actor Object Reference") (OtherComp :type "PrimitiveComponent Object Reference") (OtherBodyIndex :type Integer) (bFromSweep :type Boolean) (SweepResult :type "HitResult Structure (by ref)"))
  (bind _asmain_character (cast `/Game/Blueprints/Character/mainCharacter` OtherActor))
  (if (`self.attacking`)
    (if (not (`self.alreadyHit`))
      (`/Game/Blueprints/Character/mainCharacter.takingDamage30%` _asmain_character)
      (set `self.alreadyHit` true))))

(fn `UserConstructionScript`)