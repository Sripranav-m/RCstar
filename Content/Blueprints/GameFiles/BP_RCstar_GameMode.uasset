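; BP_RCstar_GameMode is a game mode that runs a minutes-and-seconds countdown timer and pauses the game when time runs out.
; Tick feeds a one-second Delay, which throttles the countdown to roughly one decrement of the remaining seconds per second.
; When seconds drop below zero they wrap around and a minute is subtracted, and the game pauses once the minutes go negative.
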(event `self.ReceiveTick`
  (params (DeltaSeconds :type "Float (single-precision)"))
  (`KismetSystemLibrary.Delay` 1.0)
  (set `self.remainingTime_Sec` (- (`self.remainingTime_Sec`) 1))
  (if (< (`self.remainingTime_Sec`) 0)
    (set `self.remainingTime_Sec` 59)
    (set `self.remainingTime_Min` (- (`self.remainingTime_Min`) 1))
    (if (<= (`self.remainingTime_Min`) -1)
      (`GameplayStatics.SetGamePaused` true))))

(fn `UserConstructionScript`)