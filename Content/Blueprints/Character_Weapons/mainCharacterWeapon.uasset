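; Player weapon Blueprint that handles firing and reloading for the main character.
; firingButton spawns a Projectile_base at the Muzzle socket, decrements Ammo without checking it, and plays a muzzle flash on the player's EquippedWeapon.
; Reload refills the clip from MaxAmmo, which acts as the reserve, and immediately sets the player's IsReloading flag.
; If the clip is already full, Reload writes a notice to the player's ObjectiveText instead.
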(event `firingButton`
  (`|SpawnActorFromClass` "/Game/Blueprints/Character_Weapons/projectile_base.projectile_base_C" (`SceneComponent.GetSocketTransform` (`self.weaponMesh`) "Muzzle" "RTS_World") "Undefined" "OverrideRootScale" null null)
  (set `self.Ammo` (- (`self.Ammo`) 1))
  (bind _asmain_character (cast `/Game/Blueprints/Character/mainCharacter` (`GameplayStatics.GetPlayerCharacter` 0)))
  (bind _weaponmesh (`/Game/Blueprints/Character_Weapons/mainCharacterWeapon.weaponMesh` (`/Game/Blueprints/Character/mainCharacter.equippedWeapon` _asmain_character)))
  (bind _returnvalue (`GameplayStatics.SpawnEmitterAtLocation` "/Game/InfinityBladeEffects/Effects/FX_Monsters/FX_Monster_Chicken/P_ChickenMaster_MuzzleFlash_01.P_ChickenMaster_MuzzleFlash_01" (`SceneComponent.GetSocketLocation` _weaponmesh "Muzzle") (`SceneComponent.GetSocketRotation` _weaponmesh "Muzzle") (2.0 2.0 2.0)))
  (`SceneComponent.SetWorldScale3D` _returnvalue (0.1 0.1 0.1)))

(fn `reload`
  (returns (Output_Get :type Boolean) (Output_Get1 :type Boolean))
  (locals (reloading :type "/Game/Blueprints/Character/mainCharacter Object Reference"))
  (bind _returnvalue (- (`self.clipSize`) (`self.Ammo`)))
  (if (< (`self.Ammo`) (`self.clipSize`))
    (if (>= (`self.maxAmmo`) _returnvalue)
      (set `self.ammoDifference` _returnvalue)
      (set `self.Ammo` (+ (`self.Ammo`) (`self.ammoDifference`)))
      (set `self.maxAmmo` (- (`self.maxAmmo`) (`self.ammoDifference`)))
      (bind _asmain_character (cast `/Game/Blueprints/Character/mainCharacter` (`GameplayStatics.GetPlayerCharacter` 0)))
      (bind _output_get (set `/Game/Blueprints/Character/mainCharacter.isReloading` true _asmain_character))
      (return _output_get (stale _output_get_2))
      (else
        (set `self.ammoDifference` _returnvalue)
        (set `self.Ammo` (+ (`self.Ammo`) (`self.maxAmmo`)))
        (set `self.maxAmmo` 0)
        (bind _asmain_character_2 (cast `/Game/Blueprints/Character/mainCharacter` (`GameplayStatics.GetPlayerCharacter` 0)))
        (bind _output_get_2 (set `/Game/Blueprints/Character/mainCharacter.isReloading` true _asmain_character_2))))
    (else
      (bind _asmain_character_3 (cast `/Game/Blueprints/Character/mainCharacter` (`GameplayStatics.GetPlayerCharacter` 0)))
      (set `/Game/Blueprints/Character/mainCharacter.objectiveText` "Ammo is full." _asmain_character_3))))

(fn `UserConstructionScript`)