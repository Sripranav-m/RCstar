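; E-waste pickup actor that the main character collects with the Interact input and is told to drop in a pyramid dustbin.
; EBox overlap enables input and opens a Gate for the main character, and leaving disables input and closes it.
; Interact rejects pickup if Isholding or IsholdingE is set; otherwise it sets IsholdingE and destroys itself.
; On-screen Print String messages report each result.
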(event `InputAction|Interact`
  (params (Key :type "Key Structure"))
  (:`Pressed`
    (`/Engine/EditorBlueprintResources/StandardMacros.Gate` true :!label _label
      (:`Exit`
        (bind _asmain_character (cast `/Game/Blueprints/Character/mainCharacter` (stale `self.EBox.OnComponentBeginOverlap` OtherActor)))
        (if (`/Game/Blueprints/Character/mainCharacter.isholding` _asmain_character)
          (`KismetSystemLibrary.PrintString` "Already Have an Item.." true true (struct :`R` 0.208333 :`G` 0.009029 :`B` 0.007371 :`A` 1.0) :!label _label_2)
          (else
            (bind _asmain_character_2 (cast `/Game/Blueprints/Character/mainCharacter` (stale `self.EBox.OnComponentBeginOverlap` OtherActor)))
            (if (`/Game/Blueprints/Character/mainCharacter.isholdingE` _asmain_character_2)
              (goto _label_2)
              (else
                (`KismetSystemLibrary.PrintString` "Picked up an Ewaste")
                (bind _asmain_character_3 (cast `/Game/Blueprints/Character/mainCharacter` (stale `self.EBox.OnComponentBeginOverlap` OtherActor)))
                (set `/Game/Blueprints/Character/mainCharacter.isholdingE` true _asmain_character_3)
                (`self.K2_DestroyActor`)
                (`KismetSystemLibrary.PrintString` "Drop this item in pyramid dustbin to pickup next object" true true (struct :`R` 0.013348 :`B` 0.070834 :`A` 1.0) 10.0)))))))))

(event `self.EBox.OnComponentBeginOverlap`
  (params (OverlappedComponent :type "PrimitiveComponent Object Reference") (OtherActor :type "Actor Object Reference") (OtherComp :type "PrimitiveComponent Object Reference") (OtherBodyIndex :type Integer) (bFromSweep :type Boolean) (SweepResult :type "HitResult Structure (by ref)"))
  (`self.EnableInput` (`GameplayStatics.GetPlayerController` 0))
  (cast `/Game/Blueprints/Character/mainCharacter` OtherActor)
  (goto _label :!via `Open`))

(event `self.EBox.OnComponentEndOverlap`
  (params (OverlappedComponent :type "PrimitiveComponent Object Reference") (OtherActor :type "Actor Object Reference") (OtherComp :type "PrimitiveComponent Object Reference") (OtherBodyIndex :type Integer))
  (`self.DisableInput` (`GameplayStatics.GetPlayerController` 0))
  (cast `/Game/Blueprints/Character/mainCharacter` OtherActor)
  (goto _label :!via `Close`))

(fn `UserConstructionScript`)