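; Can is a pickup actor that the player collects with the Interact input while its Box trigger is overlapped.
; Box overlap begin and end toggle the actor's input and open or close a gate on Interact, without checking which actor overlapped.
; On Interact, if the mainCharacter has neither Isholding nor IsholdingE set, it sets Isholding to true and destroys itself.
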(event `InputAction|Interact`
  (params (Key :type "Key Structure"))
  (:`Pressed`
    (`/Engine/EditorBlueprintResources/StandardMacros.Gate` true :!label _label
      (:`Exit`
        (bind _asmain_character (cast `/Game/Blueprints/Character/mainCharacter` (`GameplayStatics.GetPlayerCharacter` 0)))
        (if (not (`/Game/Blueprints/Character/mainCharacter.isholding` _asmain_character))
          (bind _asmain_character_2 (cast `/Game/Blueprints/Character/mainCharacter` (`GameplayStatics.GetPlayerCharacter` 0)))
          (if (not (`/Game/Blueprints/Character/mainCharacter.isholdingE` _asmain_character_2))
            (bind _asmain_character_3 (cast `/Game/Blueprints/Character/mainCharacter` (`GameplayStatics.GetPlayerCharacter` 0)))
            (set `/Game/Blueprints/Character/mainCharacter.isholding` true _asmain_character_3)
            (`self.K2_DestroyActor`)))))))

(event `self.Box.OnComponentBeginOverlap`
  (params (OverlappedComponent :type "PrimitiveComponent Object Reference") (OtherActor :type "Actor Object Reference") (OtherComp :type "PrimitiveComponent Object Reference") (OtherBodyIndex :type Integer) (bFromSweep :type Boolean) (SweepResult :type "HitResult Structure (by ref)"))
  (`self.EnableInput` (`GameplayStatics.GetPlayerController` 0))
  (cast `/Game/Blueprints/Character/mainCharacter` (`GameplayStatics.GetPlayerCharacter` 0))
  (goto _label :!via `Open`))

(event `self.Box.OnComponentEndOverlap`
  (params (OverlappedComponent :type "PrimitiveComponent Object Reference") (OtherActor :type "Actor Object Reference") (OtherComp :type "PrimitiveComponent Object Reference") (OtherBodyIndex :type Integer))
  (`self.DisableInput` (`GameplayStatics.GetPlayerController` 0))
  (cast `/Game/Blueprints/Character/mainCharacter` (`GameplayStatics.GetPlayerCharacter` 0))
  (goto _label :!via `Close`))

(fn `UserConstructionScript`)